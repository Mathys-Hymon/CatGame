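; Skeleton enemy master pawn that chases the nearest Player_Pawn, with a randomized movement speed set at spawn.
; StartChasing re-arms its own timer at short random intervals, finds the closest player and passes that location through ChasePlayer to ServerChase.
; ServerChase issues AI Move To toward that position.
; The AttackRange overlap event is an empty stub, so no attack happens here.
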(event OnComponentBeginOverlap(AttackRange)
  (params (OverlappedComponent :type Primitive%20Component%20Object%20Reference) (OtherActor :type Actor%20Object%20Reference) (OtherComp :type Primitive%20Component%20Object%20Reference) (OtherBodyIndex :type Integer) (bFromSweep :type Boolean) (SweepResult :type Hit%20Result%20Structure%20%28by%20ref%29)))

(event Custom|ChasePlayer
  (params (Pawn :type Pawn%20Object%20Reference) (Destination :type Vector))
  (CallFunction|ServerChase Pawn Destination))

(event Custom|ServerChase
  (params (Pawn :type Pawn%20Object%20Reference) (Destination :type Vector))
  (AI|AIMoveTo Pawn Destination 0 0.0 false))

(event Custom|StartChasing
  (bind _self self)
  (Utilities|Time|SetTimerbyEvent (delegate Custom|StartChasing) (Math|Random|RandomFloatinRange 0.05 0.3) true)
  (bind _outactors (Actor|GetAllActorsOfClass "/Game/Character/Player_Pawn.Player_Pawn_C"))
  (Utilities|IsValid (.ReturnValue (Actor|FindNearestActor (Transformation|GetActorLocation _self) _outactors))
    (:Is%20Valid
      (CallFunction|ChasePlayer _self (Transformation|GetActorLocation (.ReturnValue (Actor|FindNearestActor (Transformation|GetActorLocation _self) _outactors)))))))

(event EventBeginPlay
  (CallFunction|StartChasing)
  (Variables|/Script/Engine.FloatingPawnMovement|SetMaxSpeed (Variables|Default|GetFloatingPawnMovement) (Math|Random|RandomFloatinRange 19.0 35.0)))

(fn ConstructionScript)